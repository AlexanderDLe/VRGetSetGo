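; Test actor that pulses a cube's size and emissive glow to the audio spectrum of a sound.
; BeginPlay starts the audio, and each Tick samples a short one-band frequency spectrum of the Get_Set_Go wave at the current game time.
; That value drives actor scale plus emission strength and color in the PulseParameters material parameter collection.
; The construction script applies the EmissionPulse material and seeds the collection from the actor's variables.
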(event EventBeginPlay
  (Audio|Components|Audio|Play (Variables|Default|GetAudio) 0.0))

(event EventTick
  (params (DeltaSeconds :type Float%20%28single-precision%29))
  (bind _outspectrum (Class|SoundVisualizationStatics|CalculateFrequencySpectrum "/Game/Audio/Get_Set_Go.Get_Set_Go" 0 (Utilities|Time|GetTimeSeconds) 0.1 1))
  (Transformation|SetActorScale3D (Math|Vector|MakeVector (Utilities|Array|Get(acopy) _outspectrum) (Utilities|Array|Get(acopy) _outspectrum) (Utilities|Array|Get(acopy) _outspectrum)))
  (Rendering|Material|SetScalarParameterValue "/Game/Material/Params/PulseParameters.PulseParameters" "EmissionStrength" (Utilities|Array|Get(acopy) _outspectrum) :!class /Script/Engine.KismetMaterialLibrary)
  (Rendering|Material|SetVectorParameterValue "/Game/Material/Params/PulseParameters.PulseParameters" "Color" (Utilities|Struct|MakeLinearColor (* (Math|Float|Absolute(Float) (Utilities|Array|Get(acopy) _outspectrum)) 5.0) (* (Math|Float|Absolute(Float) (Utilities|Array|Get(acopy) _outspectrum)) 5.0) 0.0 1.0) :!class /Script/Engine.KismetMaterialLibrary))

(fn ConstructionScript
  (Rendering|Material|SetMaterial (Variables|Default|GetCube) 0 "/Game/Material/EmissionPulse.EmissionPulse")
  (Rendering|Material|SetScalarParameterValue "/Game/Material/Params/PulseParameters.PulseParameters" "EmissionStrength" (Variables|Default|GetEmissionStrength) :!class /Script/Engine.KismetMaterialLibrary)
  (Rendering|Material|SetVectorParameterValue "/Game/Material/Params/PulseParameters.PulseParameters" "Color" (Variables|Default|GetColor) :!class /Script/Engine.KismetMaterialLibrary))