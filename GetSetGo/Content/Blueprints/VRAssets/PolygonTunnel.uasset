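; An endless VR tunnel that recycles four polygon segments along Y as the player pawn passes through.
; The construction script spaces the segments by Distance and places two triggers, which hop forward along the segments on each overlap, using wrapping indices and delayed re-arming.
; FadeTrigger fades out a passed segment; RelocationTrigger moves one to the front and fades it in.
; Fades swap clockwise/counter-clockwise materials on child meshes while timelines drive the Opacity_Params collection.
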(event OnComponentBeginOverlap(RelocationTrigger)
  (params (OverlappedComponent :type Primitive%20Component%20Object%20Reference) (OtherActor :type Actor%20Object%20Reference) (OtherComp :type Primitive%20Component%20Object%20Reference) (OtherBodyIndex :type Integer) (bFromSweep :type Boolean) (SweepResult :type Hit%20Result%20Structure%20%28by%20ref%29))
  (Utilities|Casting|CastToPlayerPawn_BP OtherActor)
  (if (not (Variables|Default|GetRelocationOverlapping))
    (Utilities|FlowControl|Sequence
      (:then_0
        (Variables|Default|SetRelocationOverlapping true)
        (Transformation|SetWorldLocation (Variables|Default|GetRelocationTrigger) (Transformation|GetWorldLocation (Utilities|Array|Get(acopy) (Variables|Default|GetPolyArray) (Variables|Default|GetNextRelocationTriggerLocation))) false false))
      (:then_1
        (Transformation|SetRelativeLocation (Utilities|Array|Get(acopy) (Variables|Default|GetPolyArray) (Variables|Default|GetPolyToMoveIndex)) (Math|Vector|MakeVector 0.0 (+ (.y (Variables|/Script/Engine.SceneComponent|GetRelativeLocation (Utilities|Array|Get(acopy) (Variables|Default|GetPolyArray) (Variables|Default|GetLastPolyIndex)))) (Variables|Default|GetDistance)) 0.0) false false)
        (Utilities|FlowControl|Sequence
          (:then_0
            (bind _asstatic_mesh_component (Utilities|Casting|CastToStaticMeshComponent (Utilities|Array|Get(acopy) (Components|GetChildrenComponents (Utilities|Array|Get(acopy) (Variables|Default|GetPolyArray) (Variables|Default|GetPolyToMoveIndex)) false))))
            (Rendering|Material|SetMaterial _asstatic_mesh_component 0 (Variables|Default|GetFadeIn_CounterClockwise)))
          (:then_1
            (bind _asstatic_mesh_component_2 (Utilities|Casting|CastToStaticMeshComponent (Utilities|Array|Get(acopy) (Components|GetChildrenComponents (Utilities|Array|Get(acopy) (Variables|Default|GetPolyArray) (Variables|Default|GetPolyToMoveIndex)) false) 1)))
            (Rendering|Material|SetMaterial _asstatic_mesh_component_2 0 (Variables|Default|GetFadeIn_Clockwise)))
          (:then_2
            (bind _fadeouttimeline (Timeline|FadeIn PlayFromStart)
              (:Update
                (Rendering|Material|SetScalarParameterValue "/Game/Material/Params/Opacity_Params.Opacity_Params" "FadeIn" _fadeouttimeline :!class /Script/Engine.KismetMaterialLibrary))
              (:Finished
                (Rendering|Material|SetMaterial _asstatic_mesh_component 0 (Variables|Default|GetRotator_CounterClockwise))
                (Rendering|Material|SetMaterial _asstatic_mesh_component_2 0 (Variables|Default|GetRotator_Clockwise)))))))
      (:then_2
        (Utilities|FlowControl|Delay (Variables|Default|GetOverlapEndDelay))
        (Utilities|FlowControl|Sequence
          (:then_0
            (if (== (Variables|Default|GetNextRelocationTriggerLocation) (Variables|Default|GetMaxIndexCount))
              (Variables|Default|SetNextRelocationTriggerLocation 0)
              (else
                (Math|Integer|IncrementInt (Variables|Default|GetNextRelocationTriggerLocation)))))
          (:then_1
            (if (== (Variables|Default|GetPolyToMoveIndex) (Variables|Default|GetMaxIndexCount))
              (Variables|Default|SetPolyToMoveIndex 0)
              (else
                (Math|Integer|IncrementInt (Variables|Default|GetPolyToMoveIndex)))))
          (:then_2
            (if (== (Variables|Default|GetLastPolyIndex) (Variables|Default|GetMaxIndexCount))
              (Variables|Default|SetLastPolyIndex 0)
              (else
                (Math|Integer|IncrementInt (Variables|Default|GetLastPolyIndex)))))
          (:then_3
            (Variables|Default|SetRelocationOverlapping false)))))))

(event OnComponentBeginOverlap(FadeTrigger)
  (params (OverlappedComponent :type Primitive%20Component%20Object%20Reference) (OtherActor :type Actor%20Object%20Reference) (OtherComp :type Primitive%20Component%20Object%20Reference) (OtherBodyIndex :type Integer) (bFromSweep :type Boolean) (SweepResult :type Hit%20Result%20Structure%20%28by%20ref%29))
  (Utilities|Casting|CastToPlayerPawn_BP OtherActor)
  (if (not (Variables|Default|GetFadeOutOverlapping))
    (Utilities|FlowControl|Sequence
      (:then_0
        (Variables|Default|SetFadeOutOverlapping true)
        (Transformation|SetWorldLocation (Variables|Default|GetFadeTrigger) (Transformation|GetWorldLocation (Utilities|Array|Get(acopy) (Variables|Default|GetPolyArray) (Variables|Default|GetNextFadeTriggerLocation))) false false))
      (:then_1
        (Utilities|FlowControl|Sequence
          (:then_0
            (bind _asstatic_mesh_component (Utilities|Casting|CastToStaticMeshComponent (Utilities|Array|Get(acopy) (Components|GetChildrenComponents (Utilities|Array|Get(acopy) (Variables|Default|GetPolyArray) (Variables|Default|GetCurrentFadeIndex)) true))))
            (Rendering|Material|SetMaterial _asstatic_mesh_component 0 (Variables|Default|GetFadeOut_CounterClockwise)))
          (:then_1
            (bind _asstatic_mesh_component_2 (Utilities|Casting|CastToStaticMeshComponent (Utilities|Array|Get(acopy) (Components|GetChildrenComponents (Utilities|Array|Get(acopy) (Variables|Default|GetPolyArray) (Variables|Default|GetCurrentFadeIndex)) true) 1)))
            (Rendering|Material|SetMaterial _asstatic_mesh_component_2 0 (Variables|Default|GetFadeOut_Clockwise)))
          (:then_2
            (bind _fadeouttimeline (Timeline|FadeOut PlayFromStart)
              (:Update
                (Rendering|Material|SetScalarParameterValue "/Game/Material/Params/Opacity_Params.Opacity_Params" "FadeOut" _fadeouttimeline :!class /Script/Engine.KismetMaterialLibrary))))))
      (:then_2
        (Utilities|FlowControl|Delay (Variables|Default|GetOverlapEndDelay))
        (Utilities|FlowControl|Sequence
          (:then_0
            (if (== (Variables|Default|GetCurrentFadeIndex) (Variables|Default|GetMaxIndexCount))
              (Variables|Default|SetCurrentFadeIndex 0)
              (else
                (Math|Integer|IncrementInt (Variables|Default|GetCurrentFadeIndex)))))
          (:then_1
            (if (== (Variables|Default|GetNextFadeTriggerLocation) (Variables|Default|GetMaxIndexCount))
              (Variables|Default|SetNextFadeTriggerLocation 0)
              (else
                (Math|Integer|IncrementInt (Variables|Default|GetNextFadeTriggerLocation)))))
          (:then_2
            (Variables|Default|SetFadeOutOverlapping false)))))))

(fn ConstructionScript
  (Utilities|FlowControl|Sequence
    (:then_0
      (bind _output_get (Variables|Default|SetPolyArray (Utilities|Array|MakeArray (Variables|Default|GetPoly1) (Variables|Default|GetPoly2) (Variables|Default|GetPoly3) (Variables|Default|GetPoly4))))
      (bind _result (Math|Integer|DecrementInt (Utilities|Array|Length _output_get))
        (:%20%20
          (bind _output_get_2 (Variables|Default|SetMaxIndexCount _result))
          (Variables|Default|SetLastPolyIndex _output_get_2))))
    (:then_1
      (for _index (range 1 (Variables|Default|GetMaxIndexCount))
        (Transformation|SetRelativeLocation (Utilities|Array|Get(acopy) (Variables|Default|GetPolyArray) _index) (Math|Vector|MakeVector 0.0 (+ (.y (Variables|/Script/Engine.SceneComponent|GetRelativeLocation (Utilities|Array|Get(acopy) (Variables|Default|GetPolyArray) (- _index 1)))) (Variables|Default|GetDistance)) 0.0) false false)))
    (:then_2
      (Transformation|SetWorldLocation (Variables|Default|GetFadeTrigger) (Transformation|GetWorldLocation (Utilities|Array|Get(acopy) (Variables|Default|GetPolyArray) 1)) false false))
    (:then_3
      (Transformation|SetWorldLocation (Variables|Default|GetRelocationTrigger) (Transformation|GetWorldLocation (Utilities|Array|Get(acopy) (Variables|Default|GetPolyArray) 2)) false false))))