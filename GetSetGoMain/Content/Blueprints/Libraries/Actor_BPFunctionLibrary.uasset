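; Blueprint function library of shared helpers for a tunnel sequence driven by a player pawn timeline.
; Paired play and pause functions resume or pause the pawn's timeline, update the tunnel's rotation and materials from a start index, and optionally toggle centerpiece lasers.
; Play starts from the next fade trigger index, while pause resets materials to basic metal.
; A separate helper teleport-free moves a target to an indexed component's location.
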(fn RelocateTriggerViaChildActorCompArray
  (params (TargetToMove :type Scene%20Component%20Object%20Reference) (ComponentArray :type Array%20of%20Child%20Actor%20Component%20Object%20References) (Index :type Integer))
  (Transformation|SetWorldLocation TargetToMove (Transformation|GetWorldLocation (Utilities|Array|Get(acopy) ComponentArray Index)) false false))

(fn PauseTimelineandRotationandResetMaterials
  (params (PlayerPawn :type Player%20Pawn%20BP%20Object%20Reference) (Tunnel :type Tunnel%20BP%20Object%20Reference) (RotationLoopDelay :type Float%20%28single-precision%29) (SetMaterialLoopDelay :type Float%20%28single-precision%29) (Centerpiece :type Centerpiece%20Sphere%20Object%20Reference) (ActivateDeactivateLasers :type Boolean))
  (bind _rotationstart (Variables|/Script/GetSetGoMain.Tunnel|GetRotationStart Tunnel))
  (Default|PauseTimeline PlayerPawn)
  (Default|SetTunnelRotation Tunnel _rotationstart RotationLoopDelay 0.0 false)
  (Default|SetTunnelMaterials Tunnel "/Game/Material/Material_Instances/TriangleInstances/BasicMetal_Inst.BasicMetal_Inst" "/Game/Material/Material_Instances/TriangleInstances/BasicMetal_Inst.BasicMetal_Inst" "/Game/Material/Material_Instances/TriangleInstances/BasicMetal_Inst.BasicMetal_Inst" true SetMaterialLoopDelay _rotationstart)
  (if ActivateDeactivateLasers
    (Default|DeactivateLasers Centerpiece)))

(fn PlayTimelineandRotationandSetMaterials
  (params (PlayerPawn :type Player%20Pawn%20BP%20Object%20Reference) (Tunnel :type Tunnel%20BP%20Object%20Reference) (UnlitMaterial :type Material%20Instance%20Object%20Reference) (FadeOutMaterial :type Material%20Instance%20Object%20Reference) (FadeInMaterial :type Material%20Instance%20Object%20Reference) (ActivateMaterialsUponCompletion :type Boolean) (SetMaterialLoopDelay :type Float%20%28single-precision%29) (RotationLoopDelay :type Float%20%28single-precision%29) (RotationSpeed :type Float%20%28single-precision%29) (Clockwise :type Boolean) (Centerpiece :type Centerpiece%20Sphere%20Object%20Reference) (ActivateLasers :type Boolean))
  (bind _output_get (Variables|/Script/GetSetGoMain.Tunnel|SetRotationStart Tunnel (Variables|/Script/GetSetGoMain.Tunnel|GetNextFadeTriggerIndex Tunnel)))
  (Default|SetTunnelMaterials Tunnel UnlitMaterial FadeOutMaterial FadeInMaterial ActivateMaterialsUponCompletion SetMaterialLoopDelay _output_get)
  (Default|SetTunnelRotation Tunnel _output_get RotationLoopDelay RotationSpeed Clockwise)
  (Default|ResumeTimeline PlayerPawn)
  (if ActivateLasers
    (Default|ActivateLasers Centerpiece)))