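; Floats is a VR asset Blueprint that sets a component rotating and moving between two points.
; The StartMovement event sets the RotatingMovement rate from the RotateX, RotateY and RotateZ variables.
; It also sets the InterpToMovement control points from StartingPoint and InterpEndPoint, along with its duration.
; The RotationY input is unused, the construction script is empty, and the only StartMovement call shown never runs.
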(event Custom|StartMovement
  (params (RotationY :type Float%20%28single-precision%29))
  (bind _interptomovement (Variables|Default|GetInterpToMovement))
  (Variables|/Script/Engine.RotatingMovementComponent|SetRotationRate (Variables|Default|GetRotatingMovement) (Math|Rotator|MakeRotator (Variables|Default|GetRotateX) (Variables|Default|GetRotateY) (Variables|Default|GetRotateZ)))
  (Variables|/Script/Engine.InterpToMovementComponent|SetControlPoints _interptomovement (Utilities|Array|MakeArray (Variables|Default|GetStartingPoint) (Variables|Default|GetInterp%20End%20Point)))
  (Variables|/Script/Engine.InterpToMovementComponent|SetDuration _interptomovement (Variables|Default|GetInterpDuration)))

(fn ConstructionScript)