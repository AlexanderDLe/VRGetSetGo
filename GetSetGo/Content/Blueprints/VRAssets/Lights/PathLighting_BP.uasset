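; Path lighting actor that lights three pairs of gate lights in a staggered sequence when the player pawn enters its trigger box.
; The construction script caches six TriggerableLight_BP child actors as light references.
; On overlap by PlayerPawn_BP, a Sequence calls LightOn on each pair with a shared color and glow material, offsetting later pairs by multiples of LightDelay.
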(event OnComponentBeginOverlap(Box)
  (params (OverlappedComponent :type Primitive%20Component%20Object%20Reference) (OtherActor :type Actor%20Object%20Reference) (OtherComp :type Primitive%20Component%20Object%20Reference) (OtherBodyIndex :type Integer) (bFromSweep :type Boolean) (SweepResult :type Hit%20Result%20Structure%20%28by%20ref%29))
  (bind _bluestaticglow (Variables|Default|GetBlueStaticGlow))
  (bind _lightcolor (Variables|Default|GetLightColor))
  (Utilities|Casting|CastToPlayerPawn_BP OtherActor)
  (Utilities|FlowControl|Sequence
    (:then_0
      (Default|Lighton (Variables|Default|GetGateLight1) _lightcolor _bluestaticglow)
      (Default|Lighton (Variables|Default|GetGateLight2) _lightcolor _bluestaticglow))
    (:then_1
      (Utilities|FlowControl|Delay (Variables|Default|GetLightDelay))
      (Default|Lighton (Variables|Default|GetGateLight3) _lightcolor _bluestaticglow)
      (Default|Lighton (Variables|Default|GetGateLight4) _lightcolor _bluestaticglow))
    (:then_2
      (Utilities|FlowControl|Delay (* (Variables|Default|GetLightDelay) 2.0))
      (Default|Lighton (Variables|Default|GetGateLight5) _lightcolor _bluestaticglow)
      (Default|Lighton (Variables|Default|GetGateLight6) _lightcolor _bluestaticglow))))

(fn ConstructionScript
  (Utilities|FlowControl|Sequence
    (:then_0
      (bind _astriggerable_light_bp (Utilities|Casting|CastToTriggerableLight_BP (Variables|/Script/Engine.ChildActorComponent|GetChildActor (Variables|Default|GetGateLight_BP))))
      (Variables|Default|SetGateLight1 _astriggerable_light_bp))
    (:then_1
      (bind _astriggerable_light_bp_2 (Utilities|Casting|CastToTriggerableLight_BP (Variables|/Script/Engine.ChildActorComponent|GetChildActor (Variables|Default|GetGateLight_BP1))))
      (Variables|Default|SetGateLight2 _astriggerable_light_bp_2))
    (:then_2
      (bind _astriggerable_light_bp_3 (Utilities|Casting|CastToTriggerableLight_BP (Variables|/Script/Engine.ChildActorComponent|GetChildActor (Variables|Default|GetGateLight_BP2))))
      (Variables|Default|SetGateLight3 _astriggerable_light_bp_3))
    (:then_3
      (bind _astriggerable_light_bp_4 (Utilities|Casting|CastToTriggerableLight_BP (Variables|/Script/Engine.ChildActorComponent|GetChildActor (Variables|Default|GetGateLight_BP3))))
      (Variables|Default|SetGateLight4 _astriggerable_light_bp_4))
    (:then_4
      (bind _astriggerable_light_bp_5 (Utilities|Casting|CastToTriggerableLight_BP (Variables|/Script/Engine.ChildActorComponent|GetChildActor (Variables|Default|GetGateLight_BP4))))
      (Variables|Default|SetGateLight5 _astriggerable_light_bp_5))
    (:then_5
      (bind _astriggerable_light_bp_6 (Utilities|Casting|CastToTriggerableLight_BP (Variables|/Script/Engine.ChildActorComponent|GetChildActor (Variables|Default|GetGateLight_BP5))))
      (Variables|Default|SetGateLight6 _astriggerable_light_bp_6))))