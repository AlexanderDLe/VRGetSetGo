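; VR tunnel of evenly spaced triangle child actors that recycles itself into an endless corridor as PlayerPawn_BP passes through.
; Two leapfrogging overlap triggers advance wrapping indices: one fades out a triangle, the other moves one to the far end and fades it in.
; Timelines drive fades and glow color through Material Parameter Collections.
; Events toggle visibility, light triangles sequentially, and start staggered clockwise or counterclockwise rotation.
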(event OnComponentBeginOverlap(RelocationTrigger)
  (params (OverlappedComponent :type Primitive%20Component%20Object%20Reference) (OtherActor :type Actor%20Object%20Reference) (OtherComp :type Primitive%20Component%20Object%20Reference) (OtherBodyIndex :type Integer) (bFromSweep :type Boolean) (SweepResult :type Hit%20Result%20Structure%20%28by%20ref%29))
  (bind _polytomoveindex (Variables|Default|GetPolyToMoveIndex))
  (bind _triactorarray (Variables|Default|GetTriActorArray))
  (bind _maxindexcount (Variables|Default|GetMaxIndexCount))
  (bind _output (Utilities|Array|Get(acopy) _triactorarray _polytomoveindex))
  (Utilities|Casting|CastToPlayerPawn_BP OtherActor)
  (if (not (Variables|Default|GetRelocationOverlapping))
    (Utilities|FlowControl|Sequence
      (:then_0
        (Variables|Default|SetRelocationOverlapping true)
        (Transformation|SetWorldLocation (Variables|Default|GetRelocationTrigger) (Transformation|GetWorldLocation (Utilities|Array|Get(acopy) (Variables|Default|GetTriComponentArray) (Variables|Default|GetNextRelocationTriggerLocation))) false false))
      (:then_1
        (Transformation|SetRelativeLocation (Utilities|Array|Get(acopy) (Variables|Default|GetTriComponentArray) (Variables|Default|GetPolyToMoveIndex)) (Math|Vector|MakeVector 0.0 (+ (.y (Variables|/Script/Engine.SceneComponent|GetRelativeLocation (Utilities|Array|Get(acopy) (Variables|Default|GetTriComponentArray) (Variables|Default|GetLastPolyIndex)))) (Variables|Default|GetDistance)) 0.0) false false)
        (Utilities|FlowControl|Sequence
          (:then_0
            (Default|SetFadein _output))
          (:then_1
            (bind _fadeouttimeline (Timeline|FadeIn PlayFromStart)
              (:Update
                (Rendering|Material|SetScalarParameterValue "/Game/Material/Params/Opacity_Params.Opacity_Params" "FadeIn" _fadeouttimeline :!class /Script/Engine.KismetMaterialLibrary))
              (:Finished
                (Default|SetDefault _output))))))
      (:then_2
        (Utilities|FlowControl|Delay (Variables|Default|GetOverlapEndDelay))
        (CallFunction|IncrementandSetIndex (Variables|Default|GetNextRelocationTriggerLocation) _maxindexcount)
        (CallFunction|IncrementandSetIndex (Variables|Default|GetPolyToMoveIndex) _maxindexcount)
        (CallFunction|IncrementandSetIndex (Variables|Default|GetLastPolyIndex) _maxindexcount)
        (Variables|Default|SetRelocationOverlapping false)))))

(event OnComponentBeginOverlap(FadeTrigger)
  (params (OverlappedComponent :type Primitive%20Component%20Object%20Reference) (OtherActor :type Actor%20Object%20Reference) (OtherComp :type Primitive%20Component%20Object%20Reference) (OtherBodyIndex :type Integer) (bFromSweep :type Boolean) (SweepResult :type Hit%20Result%20Structure%20%28by%20ref%29))
  (bind _maxindexcount (Variables|Default|GetMaxIndexCount))
  (Utilities|Casting|CastToPlayerPawn_BP OtherActor)
  (if (not (Variables|Default|GetFadeOutOverlapping))
    (Utilities|FlowControl|Sequence
      (:then_0
        (Variables|Default|SetFadeOutOverlapping true)
        (Transformation|SetWorldLocation (Variables|Default|GetFadeTrigger) (Transformation|GetWorldLocation (Utilities|Array|Get(acopy) (Variables|Default|GetTriComponentArray) (Variables|Default|GetNextFadeTriggerLocation))) false false))
      (:then_1
        (Utilities|FlowControl|Sequence
          (:then_0
            (Default|SetFadeOut (Utilities|Array|Get(acopy) (Variables|Default|GetTriActorArray) (Variables|Default|GetCurrentFadeIndex))))
          (:then_1
            (bind _fadeouttimeline (Timeline|FadeOut PlayFromStart)
              (:Update
                (Rendering|Material|SetScalarParameterValue "/Game/Material/Params/Opacity_Params.Opacity_Params" "FadeOut" _fadeouttimeline :!class /Script/Engine.KismetMaterialLibrary))))))
      (:then_2
        (Utilities|FlowControl|Delay (Variables|Default|GetOverlapEndDelay))
        (CallFunction|IncrementandSetIndex (Variables|Default|GetCurrentFadeIndex) _maxindexcount)
        (CallFunction|IncrementandSetIndex (Variables|Default|GetNextFadeTriggerLocation) _maxindexcount)
        (Variables|Default|SetFadeOutOverlapping false)))))

(event Custom|ActivateTunnel
  (CallFunction|LightsON)
  (Utilities|FlowControl|Delay 1.0)
  (CallFunction|RotateClockwise))

(event Custom|ColorChange
  (params (NextColor :type Linear%20Color%20Structure))
  (bind _returnvalue (Rendering|Material|GetVectorParameterValue "/Game/Material/Params/TunnelGlow.TunnelGlow" "TunnelGlow" :!class /Script/Engine.KismetMaterialLibrary))
  (bind _colorcounter (Timeline|ColorChangeTimeline PlayFromStart)
    (:Update
      (Rendering|Material|SetVectorParameterValue "/Game/Material/Params/TunnelGlow.TunnelGlow" "TunnelGlow" (Math|Color|Lerp(LinearColor) _returnvalue NextColor _colorcounter) :!class /Script/Engine.KismetMaterialLibrary))))

(event Custom|SetRotation
  (params (RotationStart :type Integer) (LoopDelay :type Float%20%28single-precision%29) (RotationSpeed :type Float%20%28single-precision%29))
  (bind _arrayelement (Utilities|ForEachwithIndexandDelay (Variables|Default|GetTriActorArray) LoopDelay RotationStart)
    (:LoopBody
      (Default|StartRotation _arrayelement RotationSpeed))))

(event Custom|RotateCounterClockwise
  (params (StartIndex :type Integer))
  (CallFunction|SetRotation StartIndex (Variables|Default|GetRotationStartGap) (* (Variables|Default|GetRotationSpeed) -1.0)))

(event Custom|RotateClockwise
  (params (StartIndex :type Integer))
  (CallFunction|SetRotation StartIndex (Variables|Default|GetRotationStartGap) (Variables|Default|GetRotationSpeed)))

(event Custom|LightsON
  (bind _arrayelement (Utilities|ForEachwithIndexandDelay (Variables|Default|GetTriActorArray) (Variables|Default|GetLightUpSpeed))
    (:LoopBody
      (Default|StartLight _arrayelement))))

(event Custom|SetTriangleVisibility
  (params (Visibility :type Boolean))
  (for _array_element (Variables|Default|GetTriComponentArray)
    (Rendering|SetVisibility _array_element Visibility false)))

(fn ConstructionScript
  (bind _trianglecomponent5 (Variables|Default|GetTriangleComponent5))
  (bind _trianglecomponent8 (Variables|Default|GetTriangleComponent8))
  (bind _trianglecomponent9 (Variables|Default|GetTriangleComponent9))
  (bind _trianglecomponent1 (Variables|Default|GetTriangleComponent1))
  (bind _trianglecomponent2 (Variables|Default|GetTriangleComponent2))
  (bind _trianglecomponent12 (Variables|Default|GetTriangleComponent12))
  (bind _trianglecomponent10 (Variables|Default|GetTriangleComponent10))
  (bind _trianglecomponent11 (Variables|Default|GetTriangleComponent11))
  (bind _trianglecomponent13 (Variables|Default|GetTriangleComponent13))
  (bind _trianglecomponent14 (Variables|Default|GetTriangleComponent14))
  (bind _trianglecomponent3 (Variables|Default|GetTriangleComponent3))
  (bind _trianglecomponent4 (Variables|Default|GetTriangleComponent4))
  (bind _trianglecomponent0 (Variables|Default|GetTriangleComponent0))
  (bind _trianglecomponent6 (Variables|Default|GetTriangleComponent6))
  (bind _trianglecomponent7 (Variables|Default|GetTriangleComponent7))
  (Utilities|FlowControl|Sequence
    (:then_0
      (Variables|Default|SetTriComponentArray (Utilities|Array|MakeArray _trianglecomponent0 _trianglecomponent1 _trianglecomponent2 _trianglecomponent3 _trianglecomponent4 _trianglecomponent5 _trianglecomponent6 _trianglecomponent7 _trianglecomponent8 _trianglecomponent9 _trianglecomponent10 _trianglecomponent11 _trianglecomponent12 _trianglecomponent13 _trianglecomponent14)))
    (:then_1
      (Utilities|FlowControl|Sequence
        (:then_0
          (bind _astriangle_component_bp (Utilities|Casting|CastToTriangleComponent_BP (Variables|/Script/Engine.ChildActorComponent|GetChildActor _trianglecomponent0))))
        (:then_1
          (bind _astriangle_component_bp_2 (Utilities|Casting|CastToTriangleComponent_BP (Variables|/Script/Engine.ChildActorComponent|GetChildActor _trianglecomponent1))))
        (:then_2
          (bind _astriangle_component_bp_3 (Utilities|Casting|CastToTriangleComponent_BP (Variables|/Script/Engine.ChildActorComponent|GetChildActor _trianglecomponent2))))
        (:then_3
          (bind _astriangle_component_bp_4 (Utilities|Casting|CastToTriangleComponent_BP (Variables|/Script/Engine.ChildActorComponent|GetChildActor _trianglecomponent3))))
        (:then_4
          (bind _astriangle_component_bp_5 (Utilities|Casting|CastToTriangleComponent_BP (Variables|/Script/Engine.ChildActorComponent|GetChildActor _trianglecomponent4))))
        (:then_5
          (bind _astriangle_component_bp_6 (Utilities|Casting|CastToTriangleComponent_BP (Variables|/Script/Engine.ChildActorComponent|GetChildActor _trianglecomponent5))))
        (:then_6
          (bind _astriangle_component_bp_7 (Utilities|Casting|CastToTriangleComponent_BP (Variables|/Script/Engine.ChildActorComponent|GetChildActor _trianglecomponent6))))
        (:then_7
          (bind _astriangle_component_bp_8 (Utilities|Casting|CastToTriangleComponent_BP (Variables|/Script/Engine.ChildActorComponent|GetChildActor _trianglecomponent7))))
        (:then_8
          (bind _astriangle_component_bp_9 (Utilities|Casting|CastToTriangleComponent_BP (Variables|/Script/Engine.ChildActorComponent|GetChildActor _trianglecomponent8))))
        (:then_9
          (bind _astriangle_component_bp_10 (Utilities|Casting|CastToTriangleComponent_BP (Variables|/Script/Engine.ChildActorComponent|GetChildActor _trianglecomponent9))))
        (:then_10
          (bind _astriangle_component_bp_11 (Utilities|Casting|CastToTriangleComponent_BP (Variables|/Script/Engine.ChildActorComponent|GetChildActor _trianglecomponent10))))
        (:then_11
          (bind _astriangle_component_bp_12 (Utilities|Casting|CastToTriangleComponent_BP (Variables|/Script/Engine.ChildActorComponent|GetChildActor _trianglecomponent11))))
        (:then_12
          (bind _astriangle_component_bp_13 (Utilities|Casting|CastToTriangleComponent_BP (Variables|/Script/Engine.ChildActorComponent|GetChildActor _trianglecomponent12))))
        (:then_13
          (bind _astriangle_component_bp_14 (Utilities|Casting|CastToTriangleComponent_BP (Variables|/Script/Engine.ChildActorComponent|GetChildActor _trianglecomponent13))))
        (:then_14
          (bind _astriangle_component_bp_15 (Utilities|Casting|CastToTriangleComponent_BP (Variables|/Script/Engine.ChildActorComponent|GetChildActor _trianglecomponent14)))
          (Variables|Default|SetTriActorArray (Utilities|Array|MakeArray _astriangle_component_bp _astriangle_component_bp_2 _astriangle_component_bp_3 _astriangle_component_bp_4 _astriangle_component_bp_5 _astriangle_component_bp_6 _astriangle_component_bp_7 _astriangle_component_bp_8 _astriangle_component_bp_9 _astriangle_component_bp_10 _astriangle_component_bp_11 _astriangle_component_bp_12 _astriangle_component_bp_13 _astriangle_component_bp_14 _astriangle_component_bp_15)))))
    (:then_2
      (bind _result (Math|Integer|DecrementInt (Utilities|Array|Length (Variables|Default|GetTriActorArray)))
        (:%20%20
          (bind _output_get (Variables|Default|SetMaxIndexCount _result))
          (Variables|Default|SetLastPolyIndex _output_get))))
    (:then_3
      (for _index (range 1 (Variables|Default|GetMaxIndexCount))
        (Transformation|SetRelativeLocation (Utilities|Array|Get(acopy) (Variables|Default|GetTriComponentArray) _index) (Math|Vector|MakeVector 0.0 (+ (.y (Variables|/Script/Engine.SceneComponent|GetRelativeLocation (Utilities|Array|Get(acopy) (Variables|Default|GetTriComponentArray) (- _index 1)))) (Variables|Default|GetDistance)) 0.0) false false)))
    (:then_4
      (Transformation|SetWorldLocation (Variables|Default|GetFadeTrigger) (Transformation|GetWorldLocation (Utilities|Array|Get(acopy) (Variables|Default|GetTriComponentArray) 2)) false false))
    (:then_5
      (Transformation|SetWorldLocation (Variables|Default|GetRelocationTrigger) (Transformation|GetWorldLocation (Utilities|Array|Get(acopy) (Variables|Default|GetTriComponentArray) 3)) false false))))