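; SignalController is a Blueprint that drives audio-reactive visuals from kick and snare signals while a song is playing.
; Each tick it reads the signals from SignalKick and SignalSnare and uses SignalToScale to turn each into a uniform, offset and multiplied scale for its cube.
; It also writes each raw signal to an emission strength parameter in that drum's Material Parameter Collection.
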(event EventTick
  (params (DeltaSeconds :type Float%20%28single-precision%29))
  (bind _signalkick (Variables|Default|GetSignalKick))
  (bind _signalsnare (Variables|Default|GetSignalSnare))
  (bind _kicksignal (Variables|/Game/Blueprints/AudioSignals/Signal_Kick.Signal_Kick_C|GetKickSignal _signalkick))
  (bind _snaresignal (Variables|/Game/Blueprints/AudioSignals/Signal_Snare.Signal_Snare_C|GetSnareSignal _signalsnare))
  (if (Variables|Default|GetIsSongPlaying)
    (Utilities|FlowControl|Sequence
      (:then_0
        (bind _outsignal (CallFunction|SignaltoScale _kicksignal))
        (Transformation|SetActorScale3D (Variables|Default|GetCubeKick) _outsignal)
        (Rendering|Material|SetScalarParameterValue "/Game/Material/Params/Kick_Params.Kick_Params" "KickEmissionStrength" _kicksignal :!class /Script/Engine.KismetMaterialLibrary))
      (:then_1
        (bind _outsignal_2 (CallFunction|SignaltoScale _snaresignal))
        (Transformation|SetActorScale3D (Variables|Default|GetCubeSnare) _outsignal_2)
        (Rendering|Material|SetScalarParameterValue "/Game/Material/Params/Snare_Params.Snare_Params" "SnareEmissionStrength" _snaresignal :!class /Script/Engine.KismetMaterialLibrary)))))

(fn ConstructionScript)

(fn SignaltoScale
  (params (InSignal :type Float%20%28single-precision%29))
  (bind _cubescale (Variables|Default|GetCubeScale))
  (bind _decibleoffset (Variables|Default|GetDecibleOffset))
  (bind _returnvalue (+ InSignal _decibleoffset))
  (bind _returnvalue_2 (* _returnvalue _cubescale))
  (return (Math|Vector|MakeVector _returnvalue_2 _returnvalue_2 _returnvalue_2)))