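; MaterialDirector animates the tunnel glow look by driving the TunnelGlow material parameter collection.
; Three events blend glow color, band width and pan speed independently to a target over a given duration.
; Each captures the current parameter value, then lerps from it on its own timeline, with play rate set to the inverse of the duration.
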(event Custom|InterpolateTunnelColor
  (params (InterpolationLength :type Float%20%28single-precision%29) (NextColor :type Linear%20Color%20Structure))
  (bind _returnvalue (Rendering|Material|GetVectorParameterValue "/Game/Material/Params/TunnelGlow.TunnelGlow" "TunnelGlow" :!class /Script/Engine.KismetMaterialLibrary))
  (Components|Timeline|SetPlayRate (Variables|Default|GetColorChangeTimeline) (/ 1.0 InterpolationLength))
  (bind _colorcounter (Timeline|ColorChangeTimeline PlayFromStart)
    (:Update
      (Rendering|Material|SetVectorParameterValue "/Game/Material/Params/TunnelGlow.TunnelGlow" "TunnelGlow" (Math|Color|Lerp(LinearColor) _returnvalue NextColor _colorcounter) :!class /Script/Engine.KismetMaterialLibrary))))

(event Custom|InterpolateBandWidth
  (params (InterpolationLength :type Float%20%28single-precision%29) (NewWidth :type Float%20%28single-precision%29))
  (bind _returnvalue (Rendering|Material|GetScalarParameterValue "/Game/Material/Params/TunnelGlow.TunnelGlow" "WidthScalar" :!class /Script/Engine.KismetMaterialLibrary))
  (Components|Timeline|SetPlayRate (Variables|Default|GetBandWidthTimeline) (/ 1.0 InterpolationLength))
  (bind _colorcounter (Timeline|BandWidthTimeline PlayFromStart)
    (:Update
      (Rendering|Material|SetScalarParameterValue "/Game/Material/Params/TunnelGlow.TunnelGlow" "WidthScalar" (Math|Float|Lerp _returnvalue NewWidth _colorcounter) :!class /Script/Engine.KismetMaterialLibrary))))

(event Custom|InterpolateBandSpeed
  (params (InterpolationLength :type Float%20%28single-precision%29) (NewSpeed :type Float%20%28single-precision%29))
  (bind _returnvalue (Rendering|Material|GetScalarParameterValue "/Game/Material/Params/TunnelGlow.TunnelGlow" "PanSpeed" :!class /Script/Engine.KismetMaterialLibrary))
  (Components|Timeline|SetPlayRate (Variables|Default|GetPanSpeedTimeline) (/ 1.0 InterpolationLength))
  (bind _colorcounter (Timeline|PanSpeedTimeline PlayFromStart)
    (:Update
      (Rendering|Material|SetScalarParameterValue "/Game/Material/Params/TunnelGlow.TunnelGlow" "PanSpeed" (Math|Float|Lerp _returnvalue NewSpeed _colorcounter) :!class /Script/Engine.KismetMaterialLibrary))))

(fn ConstructionScript)