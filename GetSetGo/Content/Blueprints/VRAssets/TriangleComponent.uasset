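; TriangleComponent is a VR triangle prop that exposes events for spinning, lighting and fading.
; StartRotation feeds a given speed into a single axis of RotatingMovement's rotation rate.
; The other events swap materials on MergedTriangle: StartLight sets only the second slot, while the fade and default events set both the metal and triangle slots.
; Fades rely entirely on dedicated materials, with no timelines or logic in the Blueprint.
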(event Custom|StartLight
  (Rendering|Material|SetMaterial (Variables|Default|GetMergedTriangle) 1 "/Game/Material/Material_Instances/TriangleInstances/TriMat.TriMat"))

(event Custom|SetFadeOut
  (bind _mergedtriangle (Variables|Default|GetMergedTriangle))
  (Rendering|Material|SetMaterial _mergedtriangle 0 "/Game/Material/Material_Instances/TriangleInstances/MetalFadeOut.MetalFadeOut")
  (Rendering|Material|SetMaterial _mergedtriangle 1 "/Game/Material/Material_Instances/TriangleInstances/TriFadeOut.TriFadeOut"))

(event Custom|SetFadeIn
  (bind _mergedtriangle (Variables|Default|GetMergedTriangle))
  (Rendering|Material|SetMaterial _mergedtriangle 0 "/Game/Material/Material_Instances/TriangleInstances/MetalFadeIn.MetalFadeIn")
  (Rendering|Material|SetMaterial _mergedtriangle 1 "/Game/Material/Material_Instances/TriangleInstances/TriFadeIn.TriFadeIn"))

(event Custom|SetDefault
  (bind _mergedtriangle (Variables|Default|GetMergedTriangle))
  (Rendering|Material|SetMaterial _mergedtriangle 0 "/Game/Material/Masters/BasicMetal.BasicMetal")
  (Rendering|Material|SetMaterial _mergedtriangle 1 "/Game/Material/Material_Instances/TriangleInstances/TriMat.TriMat"))

(event Custom|StartRotation
  (params (RotationSpeed :type Float%20%28single-precision%29))
  (Variables|/Script/Engine.RotatingMovementComponent|SetRotationRate (Variables|Default|GetRotatingMovement) (Math|Rotator|MakeRotator 0.0 RotationSpeed 0.0)))

(fn ConstructionScript)