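; CenterpieceSphere is a sphere Blueprint that fades in as a centerpiece and then turns on its laser effect.
; FadeIn runs a timeline that drives the CenterpieceOpacity scalar in the Opacity_Params material parameter collection.
; When the fade finishes, it swaps the sphere's material to SciFi_AudioInstance and activates Lasers1, which a separate DeactivateLasers event can switch off.
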(event Custom|FadeIn
  (bind _opacity_value (Timeline|Fade%20In PlayFromStart)
    (:Update
      (Rendering|Material|SetScalarParameterValue "/Game/Material/Params/Opacity_Params.Opacity_Params" "CenterpieceOpacity" _opacity_value :!class /Script/Engine.KismetMaterialLibrary))
    (:Finished
      (Rendering|Material|SetMaterial (Variables|Default|GetCenterpieceSphere) 0 "/Game/Material/Material_Instances/FX/SciFi_AudioInstance.SciFi_AudioInstance")
      (CallFunction|ActivateLasers))))

(event Custom|ActivateLasers
  (Components|Activation|Activate (Variables|Default|GetLasers1) false))

(event Custom|DeactivateLasers
  (Components|Activation|Deactivate (Variables|Default|GetLasers1)))

(fn ConstructionScript)