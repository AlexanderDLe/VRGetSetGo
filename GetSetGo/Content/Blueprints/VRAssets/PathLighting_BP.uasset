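; PathLighting_BP is a path lighting actor that switches on six gate lights in staggered pairs when the player pawn enters its trigger box.
; The construction script casts its GateLight_BP child actors and stores them as references.
; On overlap, a sequence lights the first pair immediately, then the second and third after one and two multiples of LightDelay, creating a progressive lighting effect.
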(event OnComponentBeginOverlap(Box)
  (params (OverlappedComponent :type Primitive%20Component%20Object%20Reference) (OtherActor :type Actor%20Object%20Reference) (OtherComp :type Primitive%20Component%20Object%20Reference) (OtherBodyIndex :type Integer) (bFromSweep :type Boolean) (SweepResult :type Hit%20Result%20Structure%20%28by%20ref%29))
  (Utilities|Casting|CastToPlayerPawn_BP OtherActor)
  (Utilities|FlowControl|Sequence
    (:then_0
      (Default|Lighton (Variables|Default|GetGateLight1))
      (Default|Lighton (Variables|Default|GetGateLight2)))
    (:then_1
      (Utilities|FlowControl|Delay (Variables|Default|GetLightDelay))
      (Default|Lighton (Variables|Default|GetGateLight3))
      (Default|Lighton (Variables|Default|GetGateLight4)))
    (:then_2
      (Utilities|FlowControl|Delay (* (Variables|Default|GetLightDelay) 2.0))
      (Default|Lighton (Variables|Default|GetGateLight5))
      (Default|Lighton (Variables|Default|GetGateLight6)))))

(fn ConstructionScript
  (Utilities|FlowControl|Sequence
    (:then_0
      (bind _asgate_light_bp (Utilities|Casting|CastToGateLight_BP (Variables|/Script/Engine.ChildActorComponent|GetChildActor (Variables|Default|GetGateLight_BP))))
      (Variables|Default|SetGateLight1 _asgate_light_bp))
    (:then_1
      (bind _asgate_light_bp_2 (Utilities|Casting|CastToGateLight_BP (Variables|/Script/Engine.ChildActorComponent|GetChildActor (Variables|Default|GetGateLight_BP1))))
      (Variables|Default|SetGateLight2 _asgate_light_bp_2))
    (:then_2
      (bind _asgate_light_bp_3 (Utilities|Casting|CastToGateLight_BP (Variables|/Script/Engine.ChildActorComponent|GetChildActor (Variables|Default|GetGateLight_BP2))))
      (Variables|Default|SetGateLight3 _asgate_light_bp_3))
    (:then_3
      (bind _asgate_light_bp_4 (Utilities|Casting|CastToGateLight_BP (Variables|/Script/Engine.ChildActorComponent|GetChildActor (Variables|Default|GetGateLight_BP3))))
      (Variables|Default|SetGateLight4 _asgate_light_bp_4))
    (:then_4
      (bind _asgate_light_bp_5 (Utilities|Casting|CastToGateLight_BP (Variables|/Script/Engine.ChildActorComponent|GetChildActor (Variables|Default|GetGateLight_BP4))))
      (Variables|Default|SetGateLight5 _asgate_light_bp_5))
    (:then_5
      (bind _asgate_light_bp_6 (Utilities|Casting|CastToGateLight_BP (Variables|/Script/Engine.ChildActorComponent|GetChildActor (Variables|Default|GetGateLight_BP5))))
      (Variables|Default|SetGateLight6 _asgate_light_bp_6))))