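; Signal_Base is a base FX actor Blueprint that derives an audio signal value from a playing sound.
; CalculateAudioSignal runs only while audio plays, sampling the SoundWave's frequency spectrum over a short window at the elapsed time since AudioStartTime.
; It stores the first element of the single-band result in AudioSignal.
; Helper functions play the Audio component from the beginning and toggle actor tick.
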(fn ConstructionScript)

(fn CalculateAudioSignal
  (params (Soundwave :type Sound%20Wave%20Object%20Reference))
  (if (Variables|Default|GetIsAudioPlaying)
    (bind _outspectrum (Class|SoundVisualizationStatics|CalculateFrequencySpectrum Soundwave 0 (- (Utilities|Time|GetTimeSeconds) (Variables|Default|GetAudioStartTime)) 0.1 1))
    (Variables|Default|SetAudioSignal (Utilities|Array|Get(acopy) _outspectrum))))

(fn PlayAudio
  (Audio|Components|Audio|Play (Variables|Default|GetAudio) 0.0))

(fn EnableTick
  (params (EnableTick :type Boolean))
  (Actor|Tick|SetActorTickEnabled EnableTick))