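; Blueprint function library of shared helpers for a tunnel sequence driven by a player pawn timeline.
; Utilities advance a by-ref index that wraps to zero at a maximum and move a target to an indexed component's location.
; A pause/resume pair halts or restarts the pawn's timeline alongside tunnel rotation and material updates.
; Pausing resets tunnel materials to basic metal, while resuming applies supplied materials and rotates from the next relocation trigger location.
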(fn IncrementandSetIndex
  (params (IndexToSet :type Integer%20%28by%20ref%29) (MaxIndexCount :type Integer%20%28by%20ref%29))
  (if (== IndexToSet MaxIndexCount)
    (|SetBy-RefVar IndexToSet)
    (else
      (|SetBy-RefVar IndexToSet (+ IndexToSet 1)))))

(fn RelocateTriggerViaChildActorCompArray
  (params (TargetToMove :type Scene%20Component%20Object%20Reference) (ComponentArray :type Array%20of%20Child%20Actor%20Component%20Object%20References) (Index :type Integer))
  (Transformation|SetWorldLocation TargetToMove (Transformation|GetWorldLocation (Utilities|Array|Get(acopy) ComponentArray Index)) false false))

(fn PauseTimelineandRotationandResetMaterials
  (params (PlayerPawn :type Player%20Pawn%20BP%20Object%20Reference) (Tunnel :type Tunnel%20BP%20Object%20Reference) (RotationLoopDelay :type Float%20%28single-precision%29) (SetMaterialLoopDelay :type Float%20%28single-precision%29))
  (Default|PauseTimeline PlayerPawn)
  (Default|SetTunnelRotation Tunnel 0 RotationLoopDelay 0.0 false)
  (Default|SetTunnelMaterials Tunnel "/Game/Material/Material_Instances/TriangleInstances/BasicMetal_Inst.BasicMetal_Inst" "/Game/Material/Material_Instances/TriangleInstances/BasicMetal_Inst.BasicMetal_Inst" "/Game/Material/Material_Instances/TriangleInstances/BasicMetal_Inst.BasicMetal_Inst" true SetMaterialLoopDelay))

(fn ResumeTimelineandRotationandSetMaterials
  (params (PlayerPawn :type Player%20Pawn%20BP%20Object%20Reference) (Tunnel :type Tunnel%20BP%20Object%20Reference) (UnlitMaterial :type Material%20Instance%20Object%20Reference) (FadeOutMaterial :type Material%20Instance%20Object%20Reference) (FadeInMaterial :type Material%20Instance%20Object%20Reference) (ActivateMaterialsUponCompletion :type Boolean) (SetMaterialLoopDelay :type Float%20%28single-precision%29) (RotationLoopDelay :type Float%20%28single-precision%29) (RotationSpeed :type Float%20%28single-precision%29) (Clockwise :type Boolean))
  (Default|SetTunnelMaterials Tunnel UnlitMaterial FadeOutMaterial FadeInMaterial ActivateMaterialsUponCompletion SetMaterialLoopDelay)
  (Default|SetTunnelRotation Tunnel (Variables|/Game/Blueprints/VRAssets/Tunnel_BP.Tunnel_BP_C|GetNextRelocationTriggerLocation Tunnel) RotationLoopDelay RotationSpeed Clockwise)
  (Default|ResumeTimeline PlayerPawn))