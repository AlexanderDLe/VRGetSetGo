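; Great Hall tunnel actor built from fifteen GreatHallComponent_BP child actors, with events to set its materials and visibility.
; The construction script caches the segments, spaces them along Y by Distance, positions the relocation and fade triggers by segment index and resets each segment.
; Material events hand unlit and fade materials to every segment, then apply them through a delayed loop for a sequential light-up.
; ActivateTunnel starts that loop at LightUpSpeed, ignoring its rotation inputs.
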(event Custom|ActivateTunnel
  (params (RotationSpeed :type Float%20%28single-precision%29) (Clockwise :type Boolean))
  (CallFunction|ActivateTunnelMaterials (Variables|Default|GetLightUpSpeed)))

(event Custom|SetTunnelMaterials
  (params (UnlitMaterial :type Material%20Instance%20Object%20Reference) (FadeOutMaterial :type Material%20Instance%20Object%20Reference) (FadeInMaterial :type Material%20Instance%20Object%20Reference) (ActivateUponComplete :type Boolean) (LoopDelay :type Float%20%28single-precision%29) (StartIndex :type Integer))
  (bind _arrayelement (Utilities|ForEachwithIndexandDelay (Variables|Default|GetGreatHallChildActorComp) 0.0)
    (:LoopBody
      (Default|AssignMaterialInstances _arrayelement UnlitMaterial FadeOutMaterial FadeInMaterial))
    (:Completed
      (if ActivateUponComplete
        (CallFunction|ActivateTunnelMaterials LoopDelay StartIndex)))))

(event Custom|ActivateTunnelMaterials
  (params (LoopDelay :type Float%20%28single-precision%29) (StartIndex :type Integer))
  (bind _arrayelement (Utilities|ForEachwithIndexandDelay (Variables|Default|GetGreatHallChildActorComp) LoopDelay StartIndex)
    (:LoopBody
      (Default|SetGreatHallMaterial _arrayelement))))

(event Custom|SetTunnelVisibility
  (params (Visibility :type Boolean))
  (for _array_element (Variables|Default|GetChildActorComponentArray)
    (Rendering|SetVisibility _array_element Visibility false)))

(fn ConstructionScript
  (bind _greathallcomponent_bp1 (Variables|Default|GetGreatHallComponent_BP1))
  (bind _greathallcomponent_bp9 (Variables|Default|GetGreatHallComponent_BP9))
  (bind _greathallcomponent_bp3 (Variables|Default|GetGreatHallComponent_BP3))
  (bind _greathallcomponent_bp4 (Variables|Default|GetGreatHallComponent_BP4))
  (bind _greathallcomponent_bp5 (Variables|Default|GetGreatHallComponent_BP5))
  (bind _greathallcomponent_bp6 (Variables|Default|GetGreatHallComponent_BP6))
  (bind _greathallcomponent_bp7 (Variables|Default|GetGreatHallComponent_BP7))
  (bind _greathallcomponent_bp8 (Variables|Default|GetGreatHallComponent_BP8))
  (bind _greathallcomponent_bp2 (Variables|Default|GetGreatHallComponent_BP2))
  (bind _greathallcomponent_bp10 (Variables|Default|GetGreatHallComponent_BP10))
  (bind _greathallcomponent_bp11 (Variables|Default|GetGreatHallComponent_BP11))
  (bind _greathallcomponent_bp12 (Variables|Default|GetGreatHallComponent_BP12))
  (bind _greathallcomponent_bp13 (Variables|Default|GetGreatHallComponent_BP13))
  (bind _greathallcomponent_bp14 (Variables|Default|GetGreatHallComponent_BP14))
  (bind _greathallcomponent_bp15 (Variables|Default|GetGreatHallComponent_BP15))
  (Utilities|FlowControl|Sequence
    (:then_0
      (Variables|Default|SetChildActorComponentArray (Utilities|Array|MakeArray _greathallcomponent_bp1 _greathallcomponent_bp2 _greathallcomponent_bp3 _greathallcomponent_bp4 _greathallcomponent_bp5 _greathallcomponent_bp6 _greathallcomponent_bp7 _greathallcomponent_bp8 _greathallcomponent_bp9 _greathallcomponent_bp10 _greathallcomponent_bp11 _greathallcomponent_bp12 _greathallcomponent_bp13 _greathallcomponent_bp14 _greathallcomponent_bp15)))
    (:then_1
      (Utilities|FlowControl|Sequence
        (:then_0
          (bind _asgreat_hall_component_bp (Utilities|Casting|CastToGreatHallComponent_BP (Variables|/Script/Engine.ChildActorComponent|GetChildActor _greathallcomponent_bp1))))
        (:then_1
          (bind _asgreat_hall_component_bp_2 (Utilities|Casting|CastToGreatHallComponent_BP (Variables|/Script/Engine.ChildActorComponent|GetChildActor _greathallcomponent_bp2))))
        (:then_2
          (bind _asgreat_hall_component_bp_3 (Utilities|Casting|CastToGreatHallComponent_BP (Variables|/Script/Engine.ChildActorComponent|GetChildActor _greathallcomponent_bp3))))
        (:then_3
          (bind _asgreat_hall_component_bp_4 (Utilities|Casting|CastToGreatHallComponent_BP (Variables|/Script/Engine.ChildActorComponent|GetChildActor _greathallcomponent_bp4))))
        (:then_4
          (bind _asgreat_hall_component_bp_5 (Utilities|Casting|CastToGreatHallComponent_BP (Variables|/Script/Engine.ChildActorComponent|GetChildActor _greathallcomponent_bp5))))
        (:then_5
          (bind _asgreat_hall_component_bp_6 (Utilities|Casting|CastToGreatHallComponent_BP (Variables|/Script/Engine.ChildActorComponent|GetChildActor _greathallcomponent_bp6))))
        (:then_6
          (bind _asgreat_hall_component_bp_7 (Utilities|Casting|CastToGreatHallComponent_BP (Variables|/Script/Engine.ChildActorComponent|GetChildActor _greathallcomponent_bp7))))
        (:then_7
          (bind _asgreat_hall_component_bp_8 (Utilities|Casting|CastToGreatHallComponent_BP (Variables|/Script/Engine.ChildActorComponent|GetChildActor _greathallcomponent_bp8))))
        (:then_8
          (bind _asgreat_hall_component_bp_9 (Utilities|Casting|CastToGreatHallComponent_BP (Variables|/Script/Engine.ChildActorComponent|GetChildActor _greathallcomponent_bp9))))
        (:then_9
          (bind _asgreat_hall_component_bp_10 (Utilities|Casting|CastToGreatHallComponent_BP (Variables|/Script/Engine.ChildActorComponent|GetChildActor _greathallcomponent_bp10))))
        (:then_10
          (bind _asgreat_hall_component_bp_11 (Utilities|Casting|CastToGreatHallComponent_BP (Variables|/Script/Engine.ChildActorComponent|GetChildActor _greathallcomponent_bp11))))
        (:then_11
          (bind _asgreat_hall_component_bp_12 (Utilities|Casting|CastToGreatHallComponent_BP (Variables|/Script/Engine.ChildActorComponent|GetChildActor _greathallcomponent_bp12))))
        (:then_12
          (bind _asgreat_hall_component_bp_13 (Utilities|Casting|CastToGreatHallComponent_BP (Variables|/Script/Engine.ChildActorComponent|GetChildActor _greathallcomponent_bp13))))
        (:then_13
          (bind _asgreat_hall_component_bp_14 (Utilities|Casting|CastToGreatHallComponent_BP (Variables|/Script/Engine.ChildActorComponent|GetChildActor _greathallcomponent_bp14))))
        (:then_14
          (bind _asgreat_hall_component_bp_15 (Utilities|Casting|CastToGreatHallComponent_BP (Variables|/Script/Engine.ChildActorComponent|GetChildActor _greathallcomponent_bp15)))
          (Variables|Default|SetGreatHallChildActorComp (Utilities|Array|MakeArray _asgreat_hall_component_bp _asgreat_hall_component_bp_2 _asgreat_hall_component_bp_3 _asgreat_hall_component_bp_4 _asgreat_hall_component_bp_5 _asgreat_hall_component_bp_6 _asgreat_hall_component_bp_7 _asgreat_hall_component_bp_8 _asgreat_hall_component_bp_9 _asgreat_hall_component_bp_10 _asgreat_hall_component_bp_11 _asgreat_hall_component_bp_12 _asgreat_hall_component_bp_13 _asgreat_hall_component_bp_14 _asgreat_hall_component_bp_15)))))
    (:then_2
      (bind _result (Math|Integer|DecrementInt (Utilities|Array|Length (Variables|Default|GetGreatHallChildActorComp)))
        (:%20%20
          (bind _output_get (Variables|Default|SetMaxIndexCount _result))
          (Variables|Default|SetLastComponentIndex _output_get))))
    (:then_3
      (for _index (range 1 (Variables|Default|GetMaxIndexCount))
        (Transformation|SetRelativeLocation (Utilities|Array|Get(acopy) (Variables|Default|GetChildActorComponentArray) _index) (Math|Vector|MakeVector 0.0 (+ (.y (Variables|/Script/Engine.SceneComponent|GetRelativeLocation (Utilities|Array|Get(acopy) (Variables|Default|GetChildActorComponentArray) (- _index 1)))) (Variables|Default|GetDistance)) 0.0) false false)))
    (:then_4
      (CallFunction|RelocateTriggerViaChildActorCompArray (Variables|Default|GetRelocationTrigger) (Variables|Default|GetChildActorComponentArray) 3)
      (CallFunction|RelocateTriggerViaChildActorCompArray (Variables|Default|GetFadeTrigger) (Variables|Default|GetChildActorComponentArray) 2))
    (:then_5
      (for _array_element (Variables|Default|GetGreatHallChildActorComp)
        (Default|SetDefault _array_element)))))