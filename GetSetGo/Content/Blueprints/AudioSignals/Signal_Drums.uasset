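; Audio signal Blueprint that plays a drum track and derives a live kick signal from it.
; PlayAudio starts the DrumsAudio component from the beginning.
; While IsKickPlaying is true, Tick uses the time since KickStartTime to sample a short spectrum window of the UnrealDropTestDrums wave into KickSignal.
; Neither the playing flag nor the start time is set in this graph.
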(event Custom|PlayAudio
  (Audio|Components|Audio|Play (Variables|Default|GetDrumsAudio) 0.0))

(event EventTick
  (params (DeltaSeconds :type Float%20%28single-precision%29))
  (if (Variables|Default|GetIsKickPlaying)
    (bind _output_get (Variables|Default|SetKickTimer (- (Utilities|Time|GetTimeSeconds) (Variables|Default|GetKickStartTime))))
    (bind _outspectrum (Class|SoundVisualizationStatics|CalculateFrequencySpectrum "/Game/Audio/UnrealDropTestDrums.UnrealDropTestDrums" 0 _output_get 0.1 1))
    (Variables|Default|SetKickSignal (Utilities|Array|Get(acopy) _outspectrum))))

(fn ConstructionScript)