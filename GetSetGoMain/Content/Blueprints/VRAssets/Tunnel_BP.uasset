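; Endless VR tunnel built from fifteen triangle child actors, spaced along Y by the construction script and recycled as the player moves through.
; Player overlaps hop two triggers along the segments: one fades a segment out, the other relocates one to the tunnel's end and fades it in.
; Timelines drive the fades through a material parameter collection, with wrapping indices tracking segments.
; Events set materials, visibility and staggered activation or rotation, including alternating spin.
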(event OnComponentBeginOverlap(RelocationTrigger)
  (params (OverlappedComponent :type Primitive%20Component%20Object%20Reference) (OtherActor :type Actor%20Object%20Reference) (OtherComp :type Primitive%20Component%20Object%20Reference) (OtherBodyIndex :type Integer) (bFromSweep :type Boolean) (SweepResult :type Hit%20Result%20Structure%20%28by%20ref%29))
  (bind _triactorarray (Variables|Default|GetTriActorArray))
  (bind _componenttomoveindex (Variables|Default|GetComponentToMoveIndex))
  (bind _maxindexcount (Variables|Default|GetMaxIndexCount))
  (bind _output (Utilities|Array|Get(acopy) _triactorarray _componenttomoveindex))
  (Utilities|Casting|CastToPlayerPawn_BP OtherActor)
  (if (not (Variables|Default|GetRelocationOverlapping))
    (Utilities|FlowControl|Sequence
      (:then_0
        (Variables|Default|SetRelocationOverlapping true)
        (CallFunction|RelocateTriggerViaChildActorCompArray (Variables|Default|GetRelocationTrigger) (Variables|Default|GetTriComponentArray) (Variables|Default|GetNextRelocationTriggerIndex)))
      (:then_1
        (Class|Tunnel|RelocateComponent (Utilities|Array|Get(acopy) (Variables|Default|GetTriComponentArray) (Variables|Default|GetComponentToMoveIndex)) (Utilities|Array|Get(acopy) (Variables|Default|GetTriComponentArray) (Variables|Default|GetLastComponentIndex)) (Variables|Default|GetDistance))
        (Utilities|FlowControl|Sequence
          (:then_0
            (Default|SetFadein _output))
          (:then_1
            (bind _fadeouttimeline (Timeline|FadeIn PlayFromStart)
              (:Update
                (Rendering|Material|SetScalarParameterValue "/Game/Material/Params/Opacity_Params.Opacity_Params" "FadeIn" _fadeouttimeline :!class /Script/Engine.KismetMaterialLibrary))
              (:Finished
                (Default|SetDefault _output))))))
      (:then_2
        (Utilities|FlowControl|Delay (Variables|Default|GetOverlapDelay))
        (Class|MyBlueprintFunctionLibrary|IncrementandSetIndexCode (Variables|Default|GetNextRelocationTriggerIndex) _maxindexcount)
        (Class|MyBlueprintFunctionLibrary|IncrementandSetIndexCode (Variables|Default|GetComponentToMoveIndex) _maxindexcount)
        (Class|MyBlueprintFunctionLibrary|IncrementandSetIndexCode (Variables|Default|GetLastComponentIndex) _maxindexcount)
        (Variables|Default|SetRelocationOverlapping false)))))

(event OnComponentBeginOverlap(FadeTrigger)
  (params (OverlappedComponent :type Primitive%20Component%20Object%20Reference) (OtherActor :type Actor%20Object%20Reference) (OtherComp :type Primitive%20Component%20Object%20Reference) (OtherBodyIndex :type Integer) (bFromSweep :type Boolean) (SweepResult :type Hit%20Result%20Structure%20%28by%20ref%29))
  (bind _maxindexcount (Variables|Default|GetMaxIndexCount))
  (Utilities|Casting|CastToPlayerPawn_BP OtherActor)
  (if (not (Variables|Default|GetFadeOutOverlapping))
    (Utilities|FlowControl|Sequence
      (:then_0
        (Variables|Default|SetFadeOutOverlapping true)
        (CallFunction|RelocateTriggerViaChildActorCompArray (Variables|Default|GetFadeTrigger) (Variables|Default|GetTriComponentArray) (Variables|Default|GetNextFadeTriggerIndex)))
      (:then_1
        (Utilities|FlowControl|Sequence
          (:then_0
            (Default|SetFadeOut (Utilities|Array|Get(acopy) (Variables|Default|GetTriActorArray) (Variables|Default|GetCurrentFadeIndex))))
          (:then_1
            (bind _fadeouttimeline (Timeline|FadeOut PlayFromStart)
              (:Update
                (Rendering|Material|SetScalarParameterValue "/Game/Material/Params/Opacity_Params.Opacity_Params" "FadeOut" _fadeouttimeline :!class /Script/Engine.KismetMaterialLibrary))))))
      (:then_2
        (Utilities|FlowControl|Delay (Variables|Default|GetOverlapDelay))
        (Class|MyBlueprintFunctionLibrary|IncrementandSetIndexCode (Variables|Default|GetCurrentFadeIndex) _maxindexcount)
        (Class|MyBlueprintFunctionLibrary|IncrementandSetIndexCode (Variables|Default|GetNextFadeTriggerIndex) _maxindexcount)
        (Variables|Default|SetFadeOutOverlapping false)))))

(event Custom|ActivateTunnel
  (params (RotationLoopDelay :type Float%20%28single-precision%29) (RotationSpeed :type Float%20%28single-precision%29) (Clockwise :type Boolean))
  (CallFunction|ActivateTunnelMaterials (Variables|Default|GetLightUpSpeed))
  (Utilities|FlowControl|Delay 1.0)
  (CallFunction|SetTunnelRotation 0 RotationLoopDelay RotationSpeed Clockwise))

(event Custom|SetTunnelRotation
  (params (RotationStart :type Integer) (LoopDelay :type Float%20%28single-precision%29) (RotationSpeed :type Float%20%28single-precision%29) (Clockwise :type Boolean))
  (bind _arrayelement (Utilities|ForEachwithIndexandDelay (Variables|Default|GetTriActorArray) LoopDelay RotationStart)
    (:LoopBody
      (Default|StartRotation _arrayelement (select Clockwise RotationSpeed (* RotationSpeed -1.0))))))

(event Custom|SetTunnelMaterials
  (params (UnlitMaterial :type Material%20Instance%20Object%20Reference) (FadeOutMaterial :type Material%20Instance%20Object%20Reference) (FadeInMaterial :type Material%20Instance%20Object%20Reference) (ActivateUponComplete :type Boolean) (LoopDelay :type Float%20%28single-precision%29))
  (bind _arrayelement (Utilities|ForEachwithIndexandDelay (Variables|Default|GetTriActorArray) 0.0)
    (:LoopBody
      (Default|AssignMaterialInstances _arrayelement UnlitMaterial FadeOutMaterial FadeInMaterial))
    (:Completed
      (if ActivateUponComplete
        (CallFunction|ActivateTunnelMaterials LoopDelay)))))

(event Custom|ActivateTunnelMaterials
  (params (LoopDelay :type Float%20%28single-precision%29))
  (bind _arrayelement (Utilities|ForEachwithIndexandDelay (Variables|Default|GetTriActorArray) LoopDelay)
    (:LoopBody
      (Default|SetTriangleFrameMaterial _arrayelement))))

(event Custom|SetTunnelVisibility
  (params (Visibility :type Boolean))
  (for _array_element (Variables|Default|GetTriComponentArray)
    (Rendering|SetVisibility _array_element Visibility false)))

(event Custom|SetTunnelMixedRotation
  (params (RotationStart :type Integer) (LoopDelay :type Float%20%28single-precision%29) (RotationSpeed :type Float%20%28single-precision%29))
  (bind (_arrayelement _arrayindex) (Utilities|ForEachwithIndexandDelay (Variables|Default|GetTriActorArray) LoopDelay RotationStart)
    (:LoopBody
      (Default|StartRotation _arrayelement (select (== (Math|Integer|%(Integer) _arrayindex 2) 0) RotationSpeed (* RotationSpeed -1.0))))))

(fn ConstructionScript
  (bind _trianglecomponent5 (Variables|Default|GetTriangleComponent5))
  (bind _trianglecomponent8 (Variables|Default|GetTriangleComponent8))
  (bind _trianglecomponent9 (Variables|Default|GetTriangleComponent9))
  (bind _trianglecomponent1 (Variables|Default|GetTriangleComponent1))
  (bind _trianglecomponent2 (Variables|Default|GetTriangleComponent2))
  (bind _trianglecomponent12 (Variables|Default|GetTriangleComponent12))
  (bind _trianglecomponent10 (Variables|Default|GetTriangleComponent10))
  (bind _trianglecomponent11 (Variables|Default|GetTriangleComponent11))
  (bind _trianglecomponent13 (Variables|Default|GetTriangleComponent13))
  (bind _trianglecomponent14 (Variables|Default|GetTriangleComponent14))
  (bind _trianglecomponent3 (Variables|Default|GetTriangleComponent3))
  (bind _trianglecomponent4 (Variables|Default|GetTriangleComponent4))
  (bind _trianglecomponent0 (Variables|Default|GetTriangleComponent0))
  (bind _trianglecomponent6 (Variables|Default|GetTriangleComponent6))
  (bind _trianglecomponent7 (Variables|Default|GetTriangleComponent7))
  (Utilities|FlowControl|Sequence
    (:then_0
      (Variables|Default|SetTriComponentArray (Utilities|Array|MakeArray _trianglecomponent0 _trianglecomponent1 _trianglecomponent2 _trianglecomponent3 _trianglecomponent4 _trianglecomponent5 _trianglecomponent6 _trianglecomponent7 _trianglecomponent8 _trianglecomponent9 _trianglecomponent10 _trianglecomponent11 _trianglecomponent12 _trianglecomponent13 _trianglecomponent14)))
    (:then_1
      (Utilities|FlowControl|Sequence
        (:then_0
          (bind _astriangle_component_bp (Utilities|Casting|CastToTriangleComponent_BP (Variables|/Script/Engine.ChildActorComponent|GetChildActor _trianglecomponent0))))
        (:then_1
          (bind _astriangle_component_bp_2 (Utilities|Casting|CastToTriangleComponent_BP (Variables|/Script/Engine.ChildActorComponent|GetChildActor _trianglecomponent1))))
        (:then_2
          (bind _astriangle_component_bp_3 (Utilities|Casting|CastToTriangleComponent_BP (Variables|/Script/Engine.ChildActorComponent|GetChildActor _trianglecomponent2))))
        (:then_3
          (bind _astriangle_component_bp_4 (Utilities|Casting|CastToTriangleComponent_BP (Variables|/Script/Engine.ChildActorComponent|GetChildActor _trianglecomponent3))))
        (:then_4
          (bind _astriangle_component_bp_5 (Utilities|Casting|CastToTriangleComponent_BP (Variables|/Script/Engine.ChildActorComponent|GetChildActor _trianglecomponent4))))
        (:then_5
          (bind _astriangle_component_bp_6 (Utilities|Casting|CastToTriangleComponent_BP (Variables|/Script/Engine.ChildActorComponent|GetChildActor _trianglecomponent5))))
        (:then_6
          (bind _astriangle_component_bp_7 (Utilities|Casting|CastToTriangleComponent_BP (Variables|/Script/Engine.ChildActorComponent|GetChildActor _trianglecomponent6))))
        (:then_7
          (bind _astriangle_component_bp_8 (Utilities|Casting|CastToTriangleComponent_BP (Variables|/Script/Engine.ChildActorComponent|GetChildActor _trianglecomponent7))))
        (:then_8
          (bind _astriangle_component_bp_9 (Utilities|Casting|CastToTriangleComponent_BP (Variables|/Script/Engine.ChildActorComponent|GetChildActor _trianglecomponent8))))
        (:then_9
          (bind _astriangle_component_bp_10 (Utilities|Casting|CastToTriangleComponent_BP (Variables|/Script/Engine.ChildActorComponent|GetChildActor _trianglecomponent9))))
        (:then_10
          (bind _astriangle_component_bp_11 (Utilities|Casting|CastToTriangleComponent_BP (Variables|/Script/Engine.ChildActorComponent|GetChildActor _trianglecomponent10))))
        (:then_11
          (bind _astriangle_component_bp_12 (Utilities|Casting|CastToTriangleComponent_BP (Variables|/Script/Engine.ChildActorComponent|GetChildActor _trianglecomponent11))))
        (:then_12
          (bind _astriangle_component_bp_13 (Utilities|Casting|CastToTriangleComponent_BP (Variables|/Script/Engine.ChildActorComponent|GetChildActor _trianglecomponent12))))
        (:then_13
          (bind _astriangle_component_bp_14 (Utilities|Casting|CastToTriangleComponent_BP (Variables|/Script/Engine.ChildActorComponent|GetChildActor _trianglecomponent13))))
        (:then_14
          (bind _astriangle_component_bp_15 (Utilities|Casting|CastToTriangleComponent_BP (Variables|/Script/Engine.ChildActorComponent|GetChildActor _trianglecomponent14)))
          (Variables|Default|SetTriActorArray (Utilities|Array|MakeArray _astriangle_component_bp _astriangle_component_bp_2 _astriangle_component_bp_3 _astriangle_component_bp_4 _astriangle_component_bp_5 _astriangle_component_bp_6 _astriangle_component_bp_7 _astriangle_component_bp_8 _astriangle_component_bp_9 _astriangle_component_bp_10 _astriangle_component_bp_11 _astriangle_component_bp_12 _astriangle_component_bp_13 _astriangle_component_bp_14 _astriangle_component_bp_15)))))
    (:then_2
      (bind _result (Math|Integer|DecrementInt (Utilities|Array|Length (Variables|Default|GetTriActorArray)))
        (:%20%20
          (bind _output_get (Variables|Default|SetMaxIndexCount _result))
          (Variables|Default|SetLastComponentIndex _output_get))))
    (:then_3
      (for _index (range 1 (Variables|Default|GetMaxIndexCount))
        (Transformation|SetRelativeLocation (Utilities|Array|Get(acopy) (Variables|Default|GetTriComponentArray) _index) (Math|Vector|MakeVector 0.0 (+ (.y (Variables|/Script/Engine.SceneComponent|GetRelativeLocation (Utilities|Array|Get(acopy) (Variables|Default|GetTriComponentArray) (- _index 1)))) (Variables|Default|GetDistance)) 0.0) false false)))
    (:then_4
      (CallFunction|RelocateTriggerViaChildActorCompArray (Variables|Default|GetRelocationTrigger) (Variables|Default|GetTriComponentArray) 3)
      (CallFunction|RelocateTriggerViaChildActorCompArray (Variables|Default|GetFadeTrigger) (Variables|Default|GetTriComponentArray) 2))))