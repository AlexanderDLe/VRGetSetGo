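; FX director that drives music-reactive visuals through material parameter collections, covering glow strength and tunnel color, band width and pan speed.
; Interpolate events set a timeline's play rate from the requested length and lerp each parameter toward its new value.
; While a song plays, Tick writes audio signal values into a parameter collection and, if drum scaling is on, scales the centerpiece with the clamped drum signal.
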(event Custom|InterpolateTunnelColor
  (params (InterpolationLength :type Float%20%28single-precision%29) (NextColor :type Linear%20Color%20Structure))
  (bind _returnvalue (Rendering|Material|GetVectorParameterValue "/Game/Material/Params/TunnelGlow.TunnelGlow" "TunnelGlow" :!class /Script/Engine.KismetMaterialLibrary))
  (Components|Timeline|SetPlayRate (Variables|Default|GetColorChangeTimeline) (/ 1.0 InterpolationLength))
  (bind _colorcounter (Timeline|ColorChangeTimeline PlayFromStart)
    (:Update
      (Rendering|Material|SetVectorParameterValue "/Game/Material/Params/TunnelGlow.TunnelGlow" "TunnelGlow" (Math|Color|Lerp(LinearColor) _returnvalue NextColor _colorcounter) :!class /Script/Engine.KismetMaterialLibrary))))

(event Custom|InterpolateBandSpeed
  (params (InterpolationLength :type Float%20%28single-precision%29) (NewSpeed :type Float%20%28single-precision%29))
  (bind _returnvalue (Rendering|Material|GetScalarParameterValue "/Game/Material/Params/TunnelGlow.TunnelGlow" "PanSpeed" :!class /Script/Engine.KismetMaterialLibrary))
  (Components|Timeline|SetPlayRate (Variables|Default|GetPanSpeedTimeline) (/ 1.0 InterpolationLength))
  (bind _colorcounter (Timeline|PanSpeedTimeline PlayFromStart)
    (:Update
      (Rendering|Material|SetScalarParameterValue "/Game/Material/Params/TunnelGlow.TunnelGlow" "PanSpeed" (Math|Float|Lerp _returnvalue NewSpeed _colorcounter) :!class /Script/Engine.KismetMaterialLibrary))))

(event Custom|InterpolateBandWidth
  (params (InterpolationLength :type Float%20%28single-precision%29) (NewWidth :type Float%20%28single-precision%29))
  (bind _returnvalue (Rendering|Material|GetScalarParameterValue "/Game/Material/Params/TunnelGlow.TunnelGlow" "WidthScalar" :!class /Script/Engine.KismetMaterialLibrary))
  (Components|Timeline|SetPlayRate (Variables|Default|GetBandWidthTimeline) (/ 1.0 InterpolationLength))
  (bind _colorcounter (Timeline|BandWidthTimeline PlayFromStart)
    (:Update
      (Rendering|Material|SetScalarParameterValue "/Game/Material/Params/TunnelGlow.TunnelGlow" "WidthScalar" (Math|Float|Lerp _returnvalue NewWidth _colorcounter) :!class /Script/Engine.KismetMaterialLibrary))))

(event Custom|InterpolateEmissionStr
  (params (InterpolationLength :type Float%20%28single-precision%29) (EmissionStr :type Float%20%28single-precision%29))
  (bind _returnvalue (Rendering|Material|GetScalarParameterValue "/Game/Material/Params/Glow_Params.Glow_Params" "GlowStrength" :!class /Script/Engine.KismetMaterialLibrary))
  (Components|Timeline|SetPlayRate (Variables|Default|GetEmissionStr) (/ 1.0 InterpolationLength))
  (bind _colorcounter (Timeline|EmissionStr PlayFromStart)
    (:Update
      (Rendering|Material|SetScalarParameterValue "/Game/Material/Params/Glow_Params.Glow_Params" "GlowStrength" (Math|Float|Lerp _returnvalue EmissionStr _colorcounter) :!class /Script/Engine.KismetMaterialLibrary))))

(event EventTick
  (params (DeltaSeconds :type Float%20%28single-precision%29))
  (bind _signal_drums (Variables|Default|GetSignal_Drums))
  (bind _audiosignal (Variables|/Game/Blueprints/FX/Signal_Base.Signal_Base_C|GetAudioSignal _signal_drums))
  (if (Variables|Default|GetIsSongPlaying)
    (Utilities|FlowControl|Sequence
      (:then_0
        (if (Variables|Default|GetIsDrumScaling)
          (Rendering|Material|SetScalarParameterValue "/Game/Material/Params/AudioSignal_Params.AudioSignal_Params" "DrumSignalValue" _audiosignal :!class /Script/Engine.KismetMaterialLibrary)
          (CallFunction|ScaleObject (Variables|Default|GetCenterpiece) (/ (+ _audiosignal 2e+01) 2e+01) 1.5)))
      (:then_1
        (Rendering|Material|SetScalarParameterValue "/Game/Material/Params/AudioSignal_Params.AudioSignal_Params" "TestSignalValue" (Variables|/Game/Blueprints/FX/Signal_Base.Signal_Base_C|GetAudioSignal (Variables|Default|GetSignal_Test)) :!class /Script/Engine.KismetMaterialLibrary)))))

(fn ConstructionScript)

(fn ScaleObject
  (params (ActorToScale :type Actor%20Object%20Reference) (ScaleValue :type Float%20%28single-precision%29) (MaxValue :type Float%20%28single-precision%29))
  (bind _returnvalue (Math|Float|Clamp(Float) ScaleValue 1.0 MaxValue))
  (Transformation|SetActorScale3D ActorToScale (Math|Vector|MakeVector _returnvalue _returnvalue _returnvalue)))