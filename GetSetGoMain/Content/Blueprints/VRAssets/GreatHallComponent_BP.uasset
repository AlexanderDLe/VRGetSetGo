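; Great Hall Blueprint for VR that switches the hall's frame and solid components between default, fade-out and fade-in looks.
; AssignMaterialInstances stores the frame's unlit and fade materials, with defaults supplied by the construction script.
; Events apply these stored materials to HallFrame, while the fade and default events also give HallSolid fixed metal materials.
; The fade events only swap materials, with no timing logic in the Blueprint.
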(event Custom|SetGreatHallMaterial
  (Rendering|Material|SetMaterial (Variables|Default|GetHallFrame) 0 (Variables|Default|GetCurrentUnlitMaterial)))

(event Custom|SetFadeOut
  (Rendering|Material|SetMaterial (Variables|Default|GetHallFrame) 0 (Variables|Default|GetCurrentFadeOutMaterial))
  (Rendering|Material|SetMaterial (Variables|Default|GetHallSolid) 0 "/Game/Material/Material_Instances/TriangleInstances/MetalFadeOut.MetalFadeOut"))

(event Custom|SetFadeIn
  (Rendering|Material|SetMaterial (Variables|Default|GetHallFrame) 0 (Variables|Default|GetCurrentFadeInMaterial))
  (Rendering|Material|SetMaterial (Variables|Default|GetHallSolid) 0 "/Game/Material/Material_Instances/TriangleInstances/MetalFadeIn.MetalFadeIn"))

(event Custom|SetDefault
  (Rendering|Material|SetMaterial (Variables|Default|GetHallFrame) 0 (Variables|Default|GetCurrentUnlitMaterial))
  (Rendering|Material|SetMaterial (Variables|Default|GetHallSolid) 0 "/Game/Material/Material_Instances/TriangleInstances/BasicMetal_Inst.BasicMetal_Inst"))

(event Custom|AssignMaterialInstances
  (params (UnlitMaterial :type Material%20Instance%20Object%20Reference) (FadeOutMaterial :type Material%20Instance%20Object%20Reference) (FadeInMaterial :type Material%20Instance%20Object%20Reference))
  (Variables|Default|SetCurrentUnlitMaterial UnlitMaterial)
  (Variables|Default|SetCurrentFadeOutMaterial FadeOutMaterial)
  (Variables|Default|SetCurrentFadeInMaterial FadeInMaterial))

(fn ConstructionScript
  (CallFunction|AssignMaterialInstances "/Game/Material/Material_Instances/TriangleInstances/BasicMetal_Inst.BasicMetal_Inst" "/Game/Material/Material_Instances/TriangleInstances/TriFadeOut.TriFadeOut" "/Game/Material/Material_Instances/TriangleInstances/TriFadeIn.TriFadeIn"))