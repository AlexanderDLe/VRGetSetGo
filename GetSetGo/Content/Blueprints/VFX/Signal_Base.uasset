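; Base VFX Blueprint that derives an audio-reactive signal value from a playing sound.
; While audio plays, CalculateAudioSignal uses time elapsed since the audio start time to sample a short window of the given SoundWave.
; It runs a single-band frequency spectrum analysis on that window and stores the result as AudioSignal.
; PlayAudio starts the Audio component from the beginning.
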(fn ConstructionScript)

(fn CalculateAudioSignal
  (params (Soundwave :type Sound%20Wave%20Object%20Reference))
  (if (Variables|Default|GetIsAudioPlaying)
    (bind _output_get (Variables|Default|SetAudioTimer (- (Utilities|Time|GetTimeSeconds) (Variables|Default|GetAudioStartTime))))
    (bind _outspectrum (Class|SoundVisualizationStatics|CalculateFrequencySpectrum Soundwave 0 _output_get 0.1 1))
    (Variables|Default|SetAudioSignal (Utilities|Array|Get(acopy) _outspectrum))))

(fn PlayAudio
  (Audio|Components|Audio|Play (Variables|Default|GetAudio) 0.0))