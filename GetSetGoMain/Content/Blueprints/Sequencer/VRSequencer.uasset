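; Sequencer event Blueprint for VRSequencer that signals named stages of a timed VR sequence: intro gates, first drop and first break.
; Each event endpoint takes a bound object or interface and forwards a single matching Blueprint interface call, leaving the response to the receiver.
; The generically named SequenceEvent_0 endpoint triggers the first part of the first break.
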(fn Intro
  (params (BPI :type Sequencer%20BPI%20Interface))
  (Default|SequenceBPIIntro BPI))

(fn Intro2ndGate
  (params (BPI :type Sequencer%20BPI%20Interface))
  (Default|SequenceBPIIntro2 BPI))

(fn FirstDropPart1
  (params (BPI :type Sequencer%20BPI%20Interface))
  (Default|SequenceBPIFirstDropPart1 BPI))

(fn FirstDropPart2
  (params (BPI :type Sequencer%20BPI%20Interface))
  (Default|SequenceBPIFirstDropPart2 BPI))

(fn Intro3rdGate
  (params (BPI :type Sequencer%20BPI%20Interface))
  (Default|SequenceBPIIntro3 BPI))

(fn FirstDropPart3
  (params (BPI :type Sequencer%20BPI%20Interface))
  (Default|SequenceBPIFirstDropPart3 BPI))

(fn FirstDropPart4
  (params (BPI :type Sequencer%20BPI%20Interface))
  (Default|SequenceBPIFirstDropPart4 BPI))

(fn FirstDropEnd
  (params (BPI :type Sequencer%20BPI%20Interface))
  (Default|SequenceBPIFirstDropEnd BPI))

(fn SequenceEvent0
  (params (BPI :type Sequencer%20BPI%20Interface))
  (Default|SequenceBPIFirstBreakPart1 BPI))