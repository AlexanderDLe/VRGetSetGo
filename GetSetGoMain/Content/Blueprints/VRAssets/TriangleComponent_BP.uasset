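; TriangleComponent_BP is a VR asset for a triangle mesh that can spin and switch between default, fade-out and fade-in looks.
; The construction script caches unlit, fade-out and fade-in materials, which AssignMaterialInstances can also replace.
; Events swap those onto MergedTriangle's frame slot, with fade and default events also setting the matching metal material on the other slot.
; StartRotation sets the RotatingMovement rate around a single axis.
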(event Custom|SetTriangleFrameMaterial
  (Rendering|Material|SetMaterial (Variables|Default|GetMergedTriangle) 1 (Variables|Default|GetCurrentUnlitMaterial)))

(event Custom|SetFadeOut
  (bind _mergedtriangle (Variables|Default|GetMergedTriangle))
  (Rendering|Material|SetMaterial _mergedtriangle 1 (Variables|Default|GetCurrentFadeOutMaterial))
  (Rendering|Material|SetMaterial _mergedtriangle 0 "/Game/Material/Material_Instances/TriangleInstances/MetalFadeOut.MetalFadeOut"))

(event Custom|SetFadeIn
  (bind _mergedtriangle (Variables|Default|GetMergedTriangle))
  (Rendering|Material|SetMaterial _mergedtriangle 1 (Variables|Default|GetCurrentFadeInMaterial))
  (Rendering|Material|SetMaterial _mergedtriangle 0 "/Game/Material/Material_Instances/TriangleInstances/MetalFadeIn.MetalFadeIn"))

(event Custom|SetDefault
  (bind _mergedtriangle (Variables|Default|GetMergedTriangle))
  (Rendering|Material|SetMaterial _mergedtriangle 1 (Variables|Default|GetCurrentUnlitMaterial))
  (Rendering|Material|SetMaterial _mergedtriangle 0 "/Game/Material/Material_Instances/TriangleInstances/BasicMetal_Inst.BasicMetal_Inst"))

(event Custom|StartRotation
  (params (RotationSpeed :type Float%20%28single-precision%29))
  (Variables|/Script/Engine.RotatingMovementComponent|SetRotationRate (Variables|Default|GetRotatingMovement) (Math|Rotator|MakeRotator 0.0 RotationSpeed 0.0)))

(event Custom|AssignMaterialInstances
  (params (UnlitMaterial :type Material%20Instance%20Object%20Reference) (FadeOutMaterial :type Material%20Instance%20Object%20Reference) (FadeInMaterial :type Material%20Instance%20Object%20Reference))
  (Variables|Default|SetCurrentUnlitMaterial UnlitMaterial)
  (Variables|Default|SetCurrentFadeOutMaterial FadeOutMaterial)
  (Variables|Default|SetCurrentFadeInMaterial FadeInMaterial))

(fn ConstructionScript
  (CallFunction|AssignMaterialInstances "/Game/Material/Material_Instances/TriangleInstances/TriMat.TriMat" "/Game/Material/Material_Instances/TriangleInstances/TriFadeOut.TriFadeOut" "/Game/Material/Material_Instances/TriangleInstances/TriFadeIn.TriFadeIn"))