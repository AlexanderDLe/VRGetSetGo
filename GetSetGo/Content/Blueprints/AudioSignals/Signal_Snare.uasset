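; Audio signal Blueprint that plays a snare sound and exposes its live loudness as a SnareSignal value.
; PlayAudio starts the SnareAudio component from the beginning.
; While IsSnarePlaying is set, Tick derives elapsed time from SnareStartTime and samples a single-band frequency spectrum of the Snare wave over a short window at that offset.
; That first band becomes SnareSignal.
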(event Custom|PlayAudio
  (Audio|Components|Audio|Play (Variables|Default|GetSnareAudio) 0.0))

(event EventTick
  (params (DeltaSeconds :type Float%20%28single-precision%29))
  (if (Variables|Default|GetIsSnarePlaying)
    (bind _output_get (Variables|Default|SetSnareTimer (- (Utilities|Time|GetTimeSeconds) (Variables|Default|GetSnareStartTime))))
    (bind _outspectrum (Class|SoundVisualizationStatics|CalculateFrequencySpectrum "/Game/Audio/Snare.Snare" 0 _output_get 0.1 1))
    (Variables|Default|SetSnareSignal (Utilities|Array|Get(acopy) _outspectrum))))

(fn ConstructionScript)